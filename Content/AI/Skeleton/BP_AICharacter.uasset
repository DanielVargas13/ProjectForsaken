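; AI-controlled character, in the Skeleton AI folder, that patrols endlessly through an array of target actors.
; From BeginPlay, an AI MoveTo sends it to the current target with a small acceptance radius.
; Success and failure both advance the index and wait briefly before the next move, so a failed target is skipped.
; The index wraps to the start after the last target.
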(event `self.ReceiveBeginPlay`
  (bind _targetsindex (`self.TargetsIndex`))
  (if (>= _targetsindex (`KismetArrayLibrary.Array_Length` (`self.Targets`))) :!label _label
    (set `self.TargetsIndex` 0))
  (`|AIMoveTo` self (0.0 0.0 0.0) (`|GetArrayItem` (`self.Targets`) _targetsindex) 40.0
    (:`OnSuccess`
      _)
    (:`OnFail`
      _))
  (`/Engine/EditorBlueprintResources/StandardMacros.IncrementInt` (`self.TargetsIndex`)
    (:`  `
      (`KismetSystemLibrary.Delay` 1.0)
      (goto _label))))

(fn `UserConstructionScript`)