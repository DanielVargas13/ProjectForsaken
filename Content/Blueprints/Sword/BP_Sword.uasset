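; BP_Sword is a sword Blueprint that animates its Sword component along local Z using a float curve.
; From BeginPlay, an endless Delay-driven loop samples AnimCurve, scales the value and adds it as a local offset, then advances InTime and wraps it to zero after one.
; The offset accumulates each step, so the curve sets per-step movement rather than absolute height, at a rate not scaled by delta time.
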(event `self.ReceiveBeginPlay`
  (`SceneComponent.K2_AddLocalOffset` (`self.Sword`) (`KismetMathLibrary.MakeVector` 0.0 0.0 (* (`CurveFloat.GetFloatValue` (`self.AnimCurve`) (`self.In Time`)) 5.0)) false false :!label _label)
  (`KismetSystemLibrary.Delay` 0.02)
  (bind _output_get (set `self.In Time` (+ (`self.In Time`) 0.01)))
  (if (> _output_get 1.0)
    (set `self.In Time` 0.0)
    (goto _label)
    (else
      (goto _label))))

(fn `UserConstructionScript`)